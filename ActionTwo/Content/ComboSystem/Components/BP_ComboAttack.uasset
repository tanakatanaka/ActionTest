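; Combo attack component that builds a string from entered keys and plays the AttackData montage whose pattern matches it.
; A DoOnce gates each input until ResetToNextAttack reopens it, while railAttack plays an entry directly by index.
; Completion resets and notifies; interruption waits a tick, then restarts the combo and notifies only if the player character's active montage is not another listed attack.
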(event `AttackCombo`
  (params (targetMesh :type "SkeletalMeshComponent Object Reference"))
  (set `self.Target Mesh` targetMesh)
  (`/Engine/EditorBlueprintResources/StandardMacros.DoOnce` false :!label _label
    (:`Completed`
      (set `self.currentComboPattern` (`KismetStringLibrary.Concat_StrStr` (`self.currentComboPattern`) (`self.currentComboKey`)))
      (for _array_element (`self.attackData`) :!label _label_2
        (bind (_attackanimation _attackpattern) (break `/Game/ComboSystem/Structures/F_ComboAttack` _array_element))
        (if (`KismetStringLibrary.EqualEqual_StrStr` (`self.currentComboPattern`) _attackpattern)
          (`|PlayMontage` (`self.Target Mesh`) _attackanimation (`self.animationRate`)
            (:`then`
              (`self.BreakLoop`))
            (:`OnCompleted`
              (set `self.currentComboPattern` "")
              (`self.ResetToNextAttack` null)
              (`self.OnAttackAnimationCompleted`))
            (:`OnInterrupted`
              ;[1 1 1] If what interrupted the attack animation is an attack animation defined in the "Attack Data" variable, do not restart the combo. However, if what interrupted the attack animation is any other montage animation (roll, damage, etc.), restart the combo.
              (`KismetSystemLibrary.DelayUntilNextTick`)
              (if (not (`self.CheckIsAttackAnimation`))
                (`self.OnAttackAnimationInterrupted`)
                (set `self.currentComboPattern` "")
                (`self.ResetToNextAttack` null)))))))))

(event `ResetToNextAttack`
  (params (RestartTargetMesh :type "SkeletalMeshComponent Object Reference"))
  (set `self.Target Mesh` RestartTargetMesh)
  (goto _label :!via `Reset`))

(event `BreakLoop`
  (goto _label_2 :!via `Break`))

(event `railAttack`
  (params (targetMesh :type "SkeletalMeshComponent Object Reference") (index :type Integer))
  (set `self.Target Mesh` targetMesh)
  (`|PlayMontage` (`self.Target Mesh`) (`.attackAnimation_5_4D5CC6AA41565397ACEAECBE047327A8` (break `/Game/ComboSystem/Structures/F_ComboAttack` (`|GetArrayItem` (`self.attackData`) index))) (`self.animationRate`)
    (:`then`
      (`self.BreakLoop`))
    (:`OnCompleted`
      (`self.ResetToNextAttack` null)
      (`self.OnAttackAnimationCompleted`))
    (:`OnInterrupted`
      ;[1 1 1] If what interrupted the attack animation is an attack animation defined in the "Attack Data" variable, do not restart the combo. However, if what interrupted the attack animation is any other montage animation (roll, damage, etc.), restart the combo.
      (`KismetSystemLibrary.DelayUntilNextTick`)
      (if (not (`self.CheckIsAttackAnimation`))
        (`self.OnAttackAnimationInterrupted`)
        (set `self.currentComboPattern` "")
        (`self.ResetToNextAttack` null)))))

(fn `CheckIsAttackAnimation`
  (returns (ReturnValue :type Boolean))
  (locals (attackAnimations :type "Array of AnimMontage Object Reference"))
  (for _array_element (`self.attackData`)
    (`KismetArrayLibrary.Array_AddUnique` (`local.attackAnimations`) (`.attackAnimation_5_4D5CC6AA41565397ACEAECBE047327A8` (break `/Game/ComboSystem/Structures/F_ComboAttack` _array_element))))
  (return (`KismetArrayLibrary.Array_Contains` (`local.attackAnimations`) (`AnimInstance.GetCurrentActiveMontage` (`SkeletalMeshComponent.GetAnimInstance` (`Character.Mesh` (`GameplayStatics.GetPlayerCharacter` 0)))))))

(fn `EnterKeyAttack`
  (params (key :type String) (NewParam :type "SkeletalMeshComponent Object Reference"))
  (set `self.currentComboKey` key)
  (`self.AttackCombo` NewParam)
  (return))